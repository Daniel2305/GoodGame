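; Key pickup actor that the first-person character collects with E, recording it in the character's Keys array.
; On Box overlap, it scans that array and enables its input only if the entry at index KeyValue1 is true, gating pickup on an existing entry.
; Pressing E inserts true at KeyValue, shifting later entries rather than overwriting, then destroys the key.
; Nothing disables input when the overlap ends.
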(event `self.Box.OnComponentBeginOverlap`
  (params (OverlappedComponent :type "PrimitiveComponent Object Reference") (OtherActor :type "Actor Object Reference") (OtherComp :type "PrimitiveComponent Object Reference") (OtherBodyIndex :type Integer) (bFromSweep :type Boolean) (SweepResult :type "HitResult Structure (by ref)"))
  (bind _asfirst_person_character (cast `/Game/FirstPersonBP/Blueprints/FirstPersonCharacter` OtherActor))
  (for (_array_element _array_index) (`/Game/FirstPersonBP/Blueprints/FirstPersonCharacter.Keys` _asfirst_person_character)
    (if (and _array_element (== _array_index (`self.Key_Value_1`)))
      (`self.EnableInput` (`GameplayStatics.GetPlayerController` 0)))))

(event `Key|E`
  (params (Key :type "Key Structure"))
  (:`Pressed`
    (bind _asfirst_person_character (cast `/Game/FirstPersonBP/Blueprints/FirstPersonCharacter` (stale `self.Box.OnComponentBeginOverlap` OtherActor)))
    (`KismetArrayLibrary.Array_Insert` (`/Game/FirstPersonBP/Blueprints/FirstPersonCharacter.Keys` _asfirst_person_character) true (`self.Key_Value`))
    (`self.K2_DestroyActor`)))

(fn `UserConstructionScript`)